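; Player character Blueprint for a shooter, with keyboard-style axis and touch controls, two weapons and regenerating health.
; BeginPlay attaches an MP15 and a Glock to the Weapon socket, and ChangeWeapon toggles their visibility.
; Fire and reload act on the active weapon, while touch swipes steer the view and a double tap fires.
; Damage starts a looping regeneration timer or triggers death and destruction; save-game loading is unconnected.
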(event `InputAction|ChangeWeapon`
  (params (Key :type "Key Structure"))
  (bind _reloading (`self.Reloading`))
  (bind _rootcomponent (`Actor.RootComponent` (`self.Pistol`)))
  (bind _automat (`/Game/Blueprints/Weapon/MP15.Automat` (`self.MP15`)))
  ;[1 1 1] ChangeWeapon
  (:`Pressed`
    (`/Engine/EditorBlueprintResources/StandardMacros.FlipFlop`
      (:`A`
        (if (not _reloading)
          (set `self.EQUIPEN` false)
          (`SceneComponent.SetVisibility` _rootcomponent true false)
          (set `self.PistolEQ` true)
          (`SceneComponent.SetVisibility` _automat false false)))
      (:`B`
        (if (not _reloading)
          (set `self.EQUIPEN` true)
          (`SceneComponent.SetVisibility` _automat true true)
          (set `self.PistolEQ` false)
          (`SceneComponent.SetVisibility` _rootcomponent false false))))))

(event `self.ReceiveBeginPlay`
  (bind _mesh (`self.Mesh`))
  ;[1 1 1] Spown Weapon and Save Game
  (`|ExecutionSequence`
    (:`then_1`
      (bind _returnvalue (`|SpawnActorFromClass` "/Game/Blueprints/Weapon/MP15.MP15_C" (`KismetMathLibrary.MakeTransform` (0.0 0.0 0.0) (`KismetMathLibrary.MakeRotator` 90.0 -10.0 8.0)) "Undefined" "OverrideRootScale" null null))
      (bind _output_get (set `self.MP15` _returnvalue))
      (`self.K2_AttachToComponent` _output_get _mesh "Weapon" "SnapToTarget" "KeepRelative" "SnapToTarget" true)
      (bind _returnvalue_2 (`|SpawnActorFromClass` "/Game/Blueprints/Weapon/GlokWeapon.GlokWeapon_C" (`KismetMathLibrary.MakeTransform` (-3.0 0.0 -3.0) (struct :`Yaw` 90.0) (0.8 0.8 0.8)) "Undefined" "OverrideRootScale" null null))
      (bind _output_get_2 (set `self.Pistol` _returnvalue_2))
      (`self.K2_AttachToComponent` _output_get_2 _mesh "Weapon" "KeepRelative" "KeepRelative" "KeepRelative" true)
      (`SceneComponent.SetVisibility` (`Actor.RootComponent` (`self.Pistol`)) false false))))

(event `InputAxis|LookUp`
  (params (AxisValue :type "Float (single-precision)"))
  ;[1 1 1] Looking
  (`self.AddControllerYawInput` (* AxisValue (`GameplayStatics.GetWorldDeltaSeconds`))))

(event `InputAxis|MoveForward`
  (params (AxisValue :type "Float (single-precision)"))
  ;[1 1 1] Moving
  (`self.AddMovementInput` (`SceneComponent.GetForwardVector` (`self.CapsuleComponent`)) AxisValue))

(event `InputAxis|LookRight`
  (params (AxisValue :type "Float (single-precision)"))
  ;[1 1 1] Looking
  (`self.AddControllerPitchInput` (* AxisValue (`GameplayStatics.GetWorldDeltaSeconds`))))

(event `InputAxis|MoveRight`
  (params (AxisValue :type "Float (single-precision)"))
  ;[1 1 1] Moving
  (`self.AddMovementInput` (`SceneComponent.GetRightVector` (`self.CapsuleComponent`)) AxisValue))

(event `InputAction|Firing`
  (params (Key :type "Key Structure"))
  ;[1 1 1] LookTouch
  (:`Pressed`
    ;[1 1 1] Shooting
    (if (`self.PistolEQ`) :!label _label
      ;[1 1 1] Shooting
      (if (not (`self.Reloading`))
        (`/Game/Blueprints/Weapon/MPWeaponBase.Fire` (`self.Pistol`))
        (set `self.Fire` true))
      (elif (not (`self.Reloading`))
        (`/Game/Blueprints/Weapon/MPWeaponBase.Fire` (`self.MP15`))
        (set `self.Fire` true))))
  (:`Released`
    (set `self.Fire` false :!label _label_2)
    (if (`self.PistolEQ`)
      (`/Game/Blueprints/Weapon/GlokWeapon.Stop` (`self.Pistol`))
      (else
        (`/Game/Blueprints/Weapon/MP15.Stop` (`self.MP15`))))))

(event `self.ReceiveTick`
  (params (DeltaSeconds :type "Float (single-precision)"))
  (bind (_locationx _locationy) (`PlayerController.GetInputTouchState` (`GameplayStatics.GetPlayerController` 0) "Touch1"))
  (bind _returnvalue (`KismetMathLibrary.MakeVector2D` _locationx _locationy))
  (bind (_returnvalue_x _returnvalue_y) (`KismetMathLibrary.BreakVector2D` (* (- _returnvalue (`self.PriorLoc`)) (`self.SwipeSpeed`))))
  ;[1 1 1] LookTouch
  (`/Engine/EditorBlueprintResources/StandardMacros.Gate` true :!label _label_3
    (:`Exit`
      (if (>= (`KismetMathLibrary.VSize2D` (- _returnvalue (stale `InputAction|TouchLook` _output_get))) (`self.Swipethreshold`))
        (set `self.StartLoc` (100000.0 1000000.0))
        (`self.AddControllerYawInput` _returnvalue_x)
        (`self.AddControllerPitchInput` _returnvalue_y)
        (set `self.PriorLoc` _returnvalue)))))

(event `InputAction|TouchLook`
  (params (Key :type "Key Structure"))
  (bind (_locationx _locationy) (`PlayerController.GetInputTouchState` (`GameplayStatics.GetPlayerController` 0) "Touch1"))
  ;[1 1 1] LookTouch
  (:`Pressed`
    (bind _output_get (set `self.StartLoc` (`KismetMathLibrary.MakeVector2D` _locationx _locationy)))
    (set `self.PriorLoc` _output_get)
    (`self.DoubleClick`
      (:`Touch`
        (goto _label_3 :!via `Open`))
      (:`DoubleTouch`
        (goto _label))))
  (:`Released`
    (goto _label_2)))

(event `DamageHero`
  (params (Damage :type "Float (double-precision)"))
  ;[1 1 1] Health
  (`|ExecutionSequence`
    (:`then_0`
      (bind _output_get (set `self.CorrentHealth` (- (`self.CorrentHealth`) Damage)))
      (bind _output_get_2 (set `self.CharacterIsDead` (<= _output_get 0.99)))
      (if _output_get_2
        (`self.Death`)))
    (:`then_1`
      ;[1 1 1] ResetRestoreHealth
      (`/Engine/EditorBlueprintResources/StandardMacros.DoOnce` false :!label _label_4
        (:`Completed`
          (`KismetSystemLibrary.K2_SetTimer` null "RestoreHealth" 0.7 true))))))

(event `ResetRestoreHealth`
  ;[1 1 1] ResetRestoreHealth
  (goto _label_4 :!via `Reset`))

(event `RestoreHealth`
  ;[1 1 1] RestoreHealth
  (set `self.CorrentHealth` (+ (`self.CorrentHealth`) (`self.RestorHealth`)))
  (if (>= (`self.CorrentHealth`) (`self.TotalHealth`))
    (`KismetSystemLibrary.K2_ClearTimer` null "RestoreHealth")
    (else
      (`self.ResetRestoreHealth`))))

(event `InputAction|Reload`
  (params (Key :type "Key Structure"))
  (bind _mp15 (`self.MP15`))
  (bind _pistol (`self.Pistol`))
  (:`Pressed`
    (if true
      ;[1 1 1] Reload
      (`/Game/Blueprints/Weapon/MPWeaponBase.Reload` _mp15)
      (if (`self.PistolEQ`)
        (if (< (`/Game/Blueprints/Weapon/MPWeaponBase.AmmoCount` _pistol) (`/Game/Blueprints/Weapon/MPWeaponBase.AmmoMax` _pistol))
          (`/Engine/EditorBlueprintResources/StandardMacros.DoOnce` false :!label _label_5
            (:`Completed`
              (set `self.Reloading` true)
              (`AnimInstance.Montage_Play` (`SkeletalMeshComponent.GetAnimInstance` (`self.Mesh`)) "/Game/Blueprints/Character/MainCharacter/Animation/Reload.Reload" 1.0 "MontageLength" 0.0 true)
              (`/Game/Blueprints/Weapon/MPWeaponBase.Reload` (`self.Pistol`))
              (`KismetSystemLibrary.Delay` 1.5)
              (set `self.Reloading` false)
              (goto _label_5 :!via `Reset`))))
        (elif (< (`/Game/Blueprints/Weapon/MPWeaponBase.AmmoCount` _mp15) (`/Game/Blueprints/Weapon/MPWeaponBase.AmmoMax` _mp15))
          (`/Engine/EditorBlueprintResources/StandardMacros.DoOnce` false :!label _label_6
            (:`Completed`
              (set `self.Reloading` true)
              (`AnimInstance.Montage_Play` (`SkeletalMeshComponent.GetAnimInstance` (`self.Mesh`)) "/Game/Blueprints/Character/MainCharacter/Animation/Reload.Reload" 1.0 "MontageLength" 0.0 true)
              (`/Game/Blueprints/Weapon/MPWeaponBase.Reload` (`self.MP15`))
              (`KismetSystemLibrary.Delay` 1.5)
              (set `self.Reloading` false)
              (goto _label_6 :!via `Reset`))))))))

(event `Death`
  ;[1 1 1] Death
  (`PrimitiveComponent.SetCollisionEnabled` (`self.CapsuleComponent`) "NoCollision")
  (`SkeletalMeshComponent.PlayAnimation` (`self.Mesh`) "/Game/Blueprints/Character/MainCharacter/Animation/Death_From_Right.Death_From_Right" false)
  (`KismetSystemLibrary.Delay` 2.0)
  (`self.K2_DestroyActor`)
  (`self.K2_DestroyActor`))

(fn `Fireing`
  (bind _returnvalue (`SceneComponent.K2_GetComponentToWorld` (`Actor.RootComponent` (`self.MP15`))))
  (bind _returnvalue_2 (`|SpawnActorFromClass` "/Game/Blueprints/Effect/PLamiaGasitel.PLamiaGasitel_C" (`KismetMathLibrary.MakeTransform` (.location _returnvalue) (`KismetMathLibrary.MakeRotator` (.roll (.rotation _returnvalue)) (.pitch (.rotation _returnvalue)) (.yaw (.rotation _returnvalue)))) "Undefined" "OverrideRootScale" null null))
  (`self.SetLifeSpan` _returnvalue_2 0.08))

(fn `UserConstructionScript`)