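; Glock pistol weapon that fires hitscan shots from the player camera and damages enemies.
; Fire loops through a gate and retriggerable delay until Stop, playing an empty click without ammo.
; Each shot decrements ammo, plays sound and muzzle flash unless reloading, then traces with random spread against both enemy Blueprint types.
; Reload refills the magazine from reserve after a delay, with ammo and spread values set in the construction script.
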(event `self.Fire`
  (`|ExecutionSequence`
    (:`then_0`
      (goto _label :!via `Open`))
    (:`then_1`
      (`/Engine/EditorBlueprintResources/StandardMacros.Gate` true :!label _label
        (:`Exit`
          (`|ExecutionSequence`
            (:`then_0`
              (`KismetSystemLibrary.RetriggerableDelay` 0.3)
              (goto _label))
            (:`then_1`
              (if (> (`self.AmmoCount`) 0)
                (`self.AmmoCheck`)
                (`self.LineTrace`)
                (else
                  (`GameplayStatics.PlaySoundAtLocation` "/Game/Sound/Sound/Weapon/MP15/m4-rifle-foley-fire-selector-switch-1.m4-rifle-foley-fire-selector-switch-1" (`SceneComponent.K2_GetComponentLocation` (`self.Scene`)) (struct) 1.0 1.0 0.0 "/Game/Sound/Sound/NewSoundAttenuation.NewSoundAttenuation" "/Game/Sound/Sound/NewSoundConcurrency.NewSoundConcurrency" null))))))))))

(event `Stop`
  (goto _label :!via `Close`))

(event `self.Reload`
  (bind _returnvalue (- (`self.AmmoMax`) (`self.AmmoCount`)))
  (`GameplayStatics.PlaySoundAtLocation` "/Game/Sound/Sound/Weapon/m1911/1911-pistol-foley-magazine-replace-4.1911-pistol-foley-magazine-replace-4" (`SceneComponent.K2_GetComponentLocation` (`self.Scene`)) (struct) 1.0 1.0 0.0 "/Game/Sound/Sound/NewSoundAttenuation.NewSoundAttenuation" "/Game/Sound/Sound/NewSoundConcurrency.NewSoundConcurrency" null)
  (`KismetSystemLibrary.Delay` (`self.ReloadTme`))
  (if (== (`self.AmmoCount`) 0)
    (if (not (== (`self.AmmoInBag`) 0))
      (set `self.AmmoInBag` (- (`self.AmmoInBag`) (`self.AmmoMax`)))
      (set `self.AmmoCount` (`self.AmmoMax`)))
    (elif (== (`self.AmmoInBag`) 0)
      _
      (elif (< (`self.AmmoInBag`) (`self.AmmoMax`))
        (if (>= _returnvalue (`self.AmmoInBag`))
          (set `self.AmmoCount` (+ (`self.AmmoInBag`) (`self.AmmoCount`)))
          (set `self.AmmoInBag` 0)
          (else
            (set `self.AmmoInBag` (- (`self.AmmoInBag`) _returnvalue))
            (set `self.AmmoCount` (+ _returnvalue (`self.AmmoCount`)))))
        (else
          (set `self.AmmoInBag` (- (`self.AmmoInBag`) (- (`self.AmmoMax`) (`self.AmmoCount`))))
          (set `self.AmmoCount` (`self.AmmoMax`)))))))

(fn `AmmoCheck`
  (bind (_returnvalue_location _returnvalue_rotation) (`KismetMathLibrary.BreakTransform` (`SceneComponent.K2_GetComponentToWorld` (`self.Arrow`))))
  (`/Engine/EditorBlueprintResources/StandardMacros.DecrementInt` (`self.AmmoCount`)
    (:`  `
      (if (not (`/Game/Blueprints/Character/MainCharacter/Character_BP.Reloading` (cast `/Game/Blueprints/Character/MainCharacter/Character_BP` (`GameplayStatics.GetPlayerCharacter` 0) :!pure true)))
        (`GameplayStatics.PlaySoundAtLocation` "/Game/Sound/Sound/Weapon/m1911/1911-45cal-single-shot-processed-A.1911-45cal-single-shot-processed-A" (`self.K2_GetActorLocation`) (struct) 1.0 1.0 0.0 "/Game/Sound/Sound/NewSoundAttenuation.NewSoundAttenuation" "/Game/Sound/Sound/NewSoundConcurrency.NewSoundConcurrency" null)
        (bind _returnvalue (`|SpawnActorFromClass` "/Game/Blueprints/Effect/PLamiaGasitel.PLamiaGasitel_C" (`KismetMathLibrary.MakeTransform` _returnvalue_location _returnvalue_rotation (0.6 0.6 0.6)) "AlwaysSpawn" "OverrideRootScale" null null))
        (`self.K2_AttachToActor` _returnvalue self "SocketPistol" "SnapToTarget" "SnapToTarget" "KeepRelative" true)
        (`self.SetLifeSpan` _returnvalue 0.1)))))

(fn `LineTrace`
  (bind _bulletsrpey (`self.BulletSrpey`))
  (bind _returnvalue (* _bulletsrpey -1.0))
  (bind _camera (`/Game/Blueprints/Character/MainCharacter/Character_BP.Camera` (cast `/Game/Blueprints/Character/MainCharacter/Character_BP` (`GameplayStatics.GetPlayerCharacter` 0) :!pure true)))
  (bind _returnvalue_2 (`SceneComponent.K2_GetComponentLocation` _camera))
  (bind _outhit (`KismetSystemLibrary.LineTraceSingle` _returnvalue_2 (+ (+ _returnvalue_2 (* (`SceneComponent.GetForwardVector` _camera) 20000.0)) (`KismetMathLibrary.MakeVector` (`KismetMathLibrary.RandomFloatInRange` _returnvalue _bulletsrpey) (`KismetMathLibrary.RandomFloatInRange` _returnvalue _bulletsrpey) (`KismetMathLibrary.RandomFloatInRange` _returnvalue _bulletsrpey))) "TraceTypeQuery1"))
  (`|ExecutionSequence`
    (:`then_0`
      (bind (_bblockinghit _binitialoverlap _time _distance _location _impactpoint _normal _impactnormal _physmat _hitactor) (`GameplayStatics.BreakHitResult` _outhit))
      (bind _asenemy_2bp (cast `/Game/Blueprints/Enemy2/Police2/Enemy2BP` _hitactor))
      (`/Game/Blueprints/Enemy2/Police2/Enemy2BP.DamageEnemy` _asenemy_2bp 20.0))
    (:`then_1`
      (bind _asenemy_bp (cast `/Game/Blueprints/Enemy/Police/EnemyBP` _hitactor))
      (`/Game/Blueprints/Enemy/Police/EnemyBP.DamageEnemy` _asenemy_bp 20.0))))

(fn `UserConstructionScript`
  (`parent.UserConstructionScript`)
  (set `self.AmmoMax` 12)
  (set `self.AmmoCount` 12)
  (set `self.AmmoInBag` 70)
  (set `self.ReloadTme` 1.5)
  (set `self.BulletSrpey` 200.0))