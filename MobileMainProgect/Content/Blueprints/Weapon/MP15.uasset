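; MP15 automatic rifle Blueprint that sets its magazine, reserve ammo and spread in the construction script.
; Fire starts a looping timer behind a DoOnce, with each tick using a round until Stop or an empty magazine halts it.
; Shots trace from the player camera with negative-only random spread to damage both enemy types; only sound and muzzle effect check Reloading.
; Reload refills from the reserve after a delay.
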(event `self.Fire`
  (`/Engine/EditorBlueprintResources/StandardMacros.DoOnce` false :!label _label
    (:`Completed`
      (`KismetSystemLibrary.K2_UnPauseTimerHandle` (`self.NewVar_1`))
      (bind _returnvalue (`KismetSystemLibrary.K2_SetTimerDelegate` (delegate `CustomEvent_0`) 0.12 true))
      (set `self.NewVar_1` _returnvalue))))

(event `Stop`
  (`KismetSystemLibrary.K2_PauseTimerHandle` (`self.NewVar_1`))
  (goto _label :!via `Reset`))

(event `CustomEvent_0`
  (set `self.AmmoCount` (`KismetMathLibrary.Clamp` (- (`self.AmmoCount`) 1) 0 (`self.AmmoMax`)))
  (if (== (`self.AmmoCount`) 0)
    (`GameplayStatics.PlaySoundAtLocation` "/Game/Sound/Sound/Weapon/MP15/m4-rifle-foley-fire-selector-switch-1.m4-rifle-foley-fire-selector-switch-1" (`SceneComponent.K2_GetComponentLocation` (`self.Scene`)) (struct) 1.0 1.0 0.0 "/Game/Sound/Sound/NewSoundAttenuation.NewSoundAttenuation" "/Game/Sound/Sound/NewSoundConcurrency.NewSoundConcurrency" null)
    (`KismetSystemLibrary.K2_PauseTimerHandle` (`self.NewVar_1`))
    (`KismetSystemLibrary.K2_ClearAndInvalidateTimerHandle` (`self.NewVar_1`))
    (else
      (`self.AmmoCheck`)
      (`self.LineTrace`))))

(event `self.Reload`
  (if (`self.AbleToReload`)
    (`GameplayStatics.PlaySoundAtLocation` "/Game/Sound/Sound/Weapon/MP15/m4-rifle-foley-magazine-replace-2.m4-rifle-foley-magazine-replace-2" (`SceneComponent.K2_GetComponentLocation` (`self.Scene`)) (struct) 1.0 0.85 0.0 "/Game/Sound/Sound/NewSoundAttenuation.NewSoundAttenuation" "/Game/Sound/Sound/NewSoundConcurrency.NewSoundConcurrency" null)
    (`KismetSystemLibrary.Delay` 1.5)
    (bind _output_get (set `self.NujnChislo` (`KismetMathLibrary.Min` (- (`self.AmmoMax`) (`self.AmmoCount`)) (`self.AmmoInBag`))))
    (set `self.AmmoCount` (+ _output_get (`self.AmmoCount`)))
    (set `self.AmmoInBag` (- (`self.AmmoInBag`) (`self.NujnChislo`)))))

(fn `AmmoCheck`
  (bind _automat (`self.Automat`))
  (bind (_returnvalue_location _returnvalue_rotation) (`KismetMathLibrary.BreakTransform` (`SceneComponent.GetSocketTransform` _automat "SocketMain" "RTS_World")))
  (if (not (`/Game/Blueprints/Character/MainCharacter/Character_BP.Reloading` (cast `/Game/Blueprints/Character/MainCharacter/Character_BP` (`GameplayStatics.GetPlayerCharacter` 0) :!pure true)))
    (`GameplayStatics.PlaySoundAtLocation` "/Game/Sound/Sound/Weapon/MP15/m4-556cal-single-shot-processed-C.m4-556cal-single-shot-processed-C" (`self.K2_GetActorLocation`) (struct) 1.0 1.0 0.0 "/Game/Sound/Sound/NewSoundAttenuation.NewSoundAttenuation" "/Game/Sound/Sound/NewSoundConcurrency.NewSoundConcurrency" null)
    (`GameplayStatics.SpawnEmitterAttached` "/Game/MobileStarterContent/Particles/P_Explosion.P_Explosion" _automat "SocketMain" (0.0 0.0 0.0) _returnvalue_rotation (0.05 0.05 0.05))))

(fn `LineTrace`
  (bind _returnvalue (* (`self.BulletSrpey`) -1.0))
  (bind _camera (`/Game/Blueprints/Character/MainCharacter/Character_BP.Camera` (cast `/Game/Blueprints/Character/MainCharacter/Character_BP` (`GameplayStatics.GetPlayerCharacter` 0) :!pure true)))
  (bind _returnvalue_2 (`SceneComponent.K2_GetComponentLocation` _camera))
  (bind _outhit (`KismetSystemLibrary.LineTraceSingle` _returnvalue_2 (+ (+ _returnvalue_2 (* (`SceneComponent.GetForwardVector` _camera) 20000.0)) (`KismetMathLibrary.MakeVector` (`KismetMathLibrary.RandomFloatInRange` _returnvalue) (`KismetMathLibrary.RandomFloatInRange` _returnvalue) (`KismetMathLibrary.RandomFloatInRange` _returnvalue))) "TraceTypeQuery1"))
  (`|ExecutionSequence`
    (:`then_0`
      (bind (_bblockinghit _binitialoverlap _time _distance _location _impactpoint _normal _impactnormal _physmat _hitactor) (`GameplayStatics.BreakHitResult` _outhit))
      (bind _asenemy_2bp (cast `/Game/Blueprints/Enemy2/Police2/Enemy2BP` _hitactor))
      (`/Game/Blueprints/Enemy2/Police2/Enemy2BP.DamageEnemy` _asenemy_2bp 18.0))
    (:`then_1`
      (bind _asenemy_bp (cast `/Game/Blueprints/Enemy/Police/EnemyBP` _hitactor))
      (`/Game/Blueprints/Enemy/Police/EnemyBP.DamageEnemy` _asenemy_bp 18.0))))

(fn `UserConstructionScript`
  (`parent.UserConstructionScript`)
  (set `self.AmmoMax` 45)
  (set `self.AmmoCount` 45)
  (set `self.AmmoInBag` 200)
  (set `self.ReloadTme` 1.5)
  (set `self.BulletSrpey` 200.0))