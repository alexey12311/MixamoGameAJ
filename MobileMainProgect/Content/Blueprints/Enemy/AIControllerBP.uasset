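; AI controller for the enemy that runs the BT_BP behavior tree on BeginPlay.
; When AI perception updates on a Character_BP, it writes the sensed result to the CanSeePlayer blackboard key.
; The same event then sets HeroIsDead from the controlled EnemyBP's health and CharacterIsDead from the player character's health.
; Both death flags refresh only on these perception updates.
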(event `self.AIPerception.OnTargetPerceptionUpdated`
  (params (Actor :type "Actor Object Reference") (Stimulus :type "AIStimulus Structure"))
  (cast `/Game/Blueprints/Character/MainCharacter/Character_BP` Actor)
  (bind _output_get (set `self.CanSeePlayer` Stimulus_bSuccessfullySensed))
  (`BlackboardComponent.SetValueAsBool` (`AIBlueprintHelperLibrary.GetBlackboard` null) "CanSeePlayer" _output_get)
  (bind _asenemy_bp (cast `/Game/Blueprints/Enemy/Police/EnemyBP` (`self.K2_GetPawn`)))
  (`BlackboardComponent.SetValueAsBool` (`AIBlueprintHelperLibrary.GetBlackboard` null) "HeroIsDead" (<= (`/Game/Blueprints/Enemy/Police/EnemyBP.CorrentHealth` _asenemy_bp) 0.0))
  (bind _ascharacter_bp (cast `/Game/Blueprints/Character/MainCharacter/Character_BP` (`GameplayStatics.GetPlayerCharacter` 0)))
  (bind _output_get_2 (set `self.CharacterIsDead` (<= (`/Game/Blueprints/Character/MainCharacter/Character_BP.CorrentHealth` _ascharacter_bp) 0.0)))
  (`BlackboardComponent.SetValueAsBool` (`AIBlueprintHelperLibrary.GetBlackboard` null) "CharacterIsDead" _output_get_2))

(event `self.ReceiveBeginPlay`
  (`self.RunBehaviorTree` "/Game/Blueprints/Enemy/BT_BP.BT_BP"))

(fn `UserConstructionScript`)