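; Respawn_BP is a checkpoint trigger that saves the player character's location when it overlaps the box.
; On overlap by a Character_BP, it loads the existing save slot or creates a new SaveGameBP object if none exists.
; It writes the character's current location to LastLocation and saves back to the same slot.
; The file only records the location; it contains no respawn logic itself.
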(event `self.Box.OnComponentBeginOverlap`
  (params (OverlappedComponent :type "PrimitiveComponent Object Reference") (OtherActor :type "Actor Object Reference") (OtherComp :type "PrimitiveComponent Object Reference") (OtherBodyIndex :type Integer) (bFromSweep :type Boolean) (SweepResult :type "HitResult Structure (by ref)"))
  (bind _savesubobject (`self.SaveSubObject`))
  (bind _location (`self.Location`))
  (bind _ascharacter_bp (cast `/Game/Blueprints/Character/MainCharacter/Character_BP` OtherActor))
  (set `self.Location` (`self.K2_GetActorLocation` _ascharacter_bp))
  (bind _returnvalue (`GameplayStatics.DoesSaveGameExist` "SlotName"))
  (if _returnvalue
    (bind _returnvalue_2 (`GameplayStatics.LoadGameFromSlot` "SlotName"))
    (bind _output_get (set `self.SaveSubObject` _returnvalue_2))
    (bind _assave_game_bp (cast `/Game/Blueprints/SaveGameBP` _output_get))
    (set `/Game/Blueprints/SaveGameBP.LastLocation` _location _assave_game_bp)
    (`GameplayStatics.SaveGameToSlot` _savesubobject "SlotName")
    (else
      (bind _returnvalue_3 (`GameplayStatics.CreateSaveGameObject` "/Game/Blueprints/SaveGameBP.SaveGameBP_C"))
      (bind _output_get_2 (set `self.SaveSubObject` _returnvalue_3))
      (bind _assave_game_bp_2 (cast `/Game/Blueprints/SaveGameBP` _output_get_2))
      (set `/Game/Blueprints/SaveGameBP.LastLocation` _location _assave_game_bp_2)
      (`GameplayStatics.SaveGameToSlot` _savesubobject "SlotName"))))

(fn `UserConstructionScript`)